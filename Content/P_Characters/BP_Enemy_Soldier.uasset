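; Enemy soldier character that acquires the player as its target when it sees or is damaged by them.
; On BeginPlay it spawns and possesses itself with a BP_AI_Controller, runs BT_Enemy_Soldier and binds to its HealthComponent's damage delegate.
; PawnSensing and damage events both feed CheckTargetPlayer, which accepts only a PlayerCharacter.
; If no valid Target exists, it writes the player to the blackboard and sets AI focus.
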(event OnSeePawn(PawnSensingComponent)
  (params (Pawn :type Pawn%20Object%20Reference))
  (CallFunction|CheckTargetPlayer Pawn))

(event Custom|OnDamageTaken
  (params (Damage :type Float%20%28single-precision%29) (CurrentHealth :type Float%20%28single-precision%29) (MaxHealth :type Float%20%28single-precision%29) (Instigator :type Actor%20Object%20Reference))
  (CallFunction|CheckTargetPlayer Instigator))

(event EventBeginPlay
  (bind _returnvalue (Game|SpawnActorfromClass "/Game/P_AI/BP_AI_Controller.BP_AI_Controller_C" (Math|Transform|MakeTransform "0, 0, 0" "0, 0, 0" "1.000000,1.000000,1.000000") "Undefined" "MultiplyWithRoot" 0 0))
  (Pawn|Possess _returnvalue self)
  (AI|RunBehaviorTree _returnvalue "/Game/P_AI/BT_Enemy_Soldier.BT_Enemy_Soldier")
  (EventDispatchers|AssignOnDamageTakenDelegate (Variables|Default|GetHealthComponent) (delegate Custom|OnDamageTaken)))

(event Collision|EventActorBeginOverlap
  (params (OtherActor :type Actor%20Object%20Reference)))

(event EventTick
  (params (DeltaSeconds :type Float%20%28single-precision%29)))

(fn ConstructionScript)

(fn CheckTargetPlayer
  (params (Instigator :type Object%20Object%20Reference))
  (bind _returnvalue (AI|GetBlackboard 0))
  (bind _returnvalue_2 (Utilities|Name|MakeLiteralName "Target"))
  (bind _self self)
  (bind _returnvalue_3 (AI|GetAIController _self))
  (bind _asplayer_character (Utilities|Casting|CastToPlayerCharacter Instigator))
  (Utilities|IsValid (AI|Components|Blackboard|GetValueasObject _returnvalue _returnvalue_2)
    (:Is%20Not%20Valid
      (AI|Components|Blackboard|SetValueasObject _returnvalue _returnvalue_2 _asplayer_character)
      (Utilities|IsValid _returnvalue_3
        (:Is%20Valid
          (AI|SetFocus _returnvalue_3 _asplayer_character))))))